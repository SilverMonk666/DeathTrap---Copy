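; GM_Tester is a game mode that handles level start and player respawn state.
; On BeginPlay it records the first keycard's transform and spawns a BP_AnimalBase AI at every SpawnersAI actor.
; On player restart it respawns a missing keycard at that transform.
; A separate custom event restores the player character's inventory, held item and keycard from stored references, and resets the countdown if it has finished.
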(event Custom|RespawnPlayer
  ;[1 1 1] Setting All variables back on respawning Playr
)

(event Custom|Spawn
  (bind _outactors (Actor|GetAllActorsOfClass "/Game/Objects/Blueprints/Logic/SpawnersAI.SpawnersAI_C"))
  (for _array_element _outactors
    (AI|SpawnAIFromClass "/Game/Characters/Animals/BP_AnimalBase.BP_AnimalBase_C" 0 (Transformation|GetWorldLocation (Variables|/Game/Objects/Blueprints/Logic/SpawnersAI.SpawnersAI_C|GetDefaultSceneRoot _array_element)) "0, 0, 0" false)))

(event Custom|CustomEvent
  (params (NewPlayer :type Controller%20Object%20Reference))
  (bind _inventoryref (Variables|Default|GetInventoryRef))
  ;[1 1 1] Setting All variables back on respawning Playr
  (Utilities|IsValid NewPlayer
    (:Is%20Valid
      (bind _asphase_player_character (Utilities|Casting|CastToPhasePlayerCharacter (Game|GetPlayerCharacter 0)))
      (Variables|/Game/BlueprintCharacters/PhasePlayerCharacter.PhasePlayerCharacter_C|SetInventory _asphase_player_character _inventoryref)
      (bind _output_get (Variables|Default|SetInHand (Utilities|Array|Get(acopy) _inventoryref)))
      (Variables|/Game/BlueprintCharacters/PhasePlayerCharacter.PhasePlayerCharacter_C|SetItemInHand _asphase_player_character _output_get)
      (Variables|/Game/BlueprintCharacters/PhasePlayerCharacter.PhasePlayerCharacter_C|SetKeyCard01 _asphase_player_character (Variables|Default|GetKeycard01Ref))
      (if (Variables|Default|GetTimerDone?)
        (Variables|Default|SetTimerDone? false)
        (Variables|Default|SetMinutes 0)
        (Variables|Default|SetSeconds 20)))))

(event EventBeginPlay
  (bind _outactors (Actor|GetAllActorsOfClass "/Game/Objects/Blueprints/BP_Interacts/BP_KeyCard.BP_KeyCard_C"))
  (Variables|Default|SetTransform (Transformation|GetActorTransform (Utilities|Array|Get(acopy) _outactors)))
  (Variables|Default|SetGameStarted true)
  (CallFunction|Spawn))

(event EventTick
  (params (DeltaSeconds :type Float%20%28single-precision%29)))

(event EventOnRestartPlayer
  (params (NewPlayer :type Controller%20Object%20Reference))
  (if (Variables|Default|GetGameStarted)
    (bind _outactors (Actor|GetAllActorsOfClass "/Game/Objects/Blueprints/BP_Interacts/BP_KeyCard.BP_KeyCard_C"))
    (Utilities|IsValid (Utilities|Array|Get(acopy) _outactors)
      (:Is%20Not%20Valid
        (Game|SpawnActorfromClass "/Game/Objects/Blueprints/BP_Interacts/BP_KeyCard.BP_KeyCard_C" (Variables|Default|GetTransform) "Undefined" 0 0)))))

(fn ConstructionScript)