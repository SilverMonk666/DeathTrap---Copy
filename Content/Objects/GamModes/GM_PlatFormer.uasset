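; Platformer game mode that creates the keycard HUD, spawns AI animals at spawner actors and handles respawning at checkpoints.
; RespawnPlayer destroys the animals, spawns and possesses a new climber character at the checkpoint in the active state, respawns AI, and resets moving platforms and pressure plates.
; On player restart it restores saved inventory, held item and keycard to the character and resets the countdown if it has expired.
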(event Custom|RespawnPlayer
  ;[1 1 1] Respawning System
  ;;[1 1 1] Destroy AI
  (bind _outactors (Actor|GetAllActorsOfClass "/Game/Characters/Animals/BP_AnimalBase.BP_AnimalBase_C"))
  (for _array_element _outactors
    (Actor|DestroyActor _array_element))
  (Utilities|FlowControl|Sequence
    (:then_0
      ;;[1 1 1] Find Active Checkpoint
      (bind _outactors_2 (Actor|GetAllActorsOfClass "/Game/Objects/Blueprints/BP_InteractiveCheckPoint.BP_InteractiveCheckPoint_C"))
      (bind _array_element_2 (Utilities|Array|ForEachLoopwithBreak _outactors_2 :!label _label)
        (:LoopBody
          (if (Utilities|Enum|Equal(Enum) (Variables|/Game/Objects/Blueprints/BP_InteractiveCheckPoint.BP_InteractiveCheckPoint_C|GetOnOffState _array_element_2) "NewEnumerator0")
            (goto _label Break)))
        (:Completed
          (bind _output_get (Variables|Default|SetCheckPoints _array_element_2))
          ;;[1 1 1] Spawn Player
          (bind _returnvalue (Game|SpawnActorfromClass "/Game/BlueprintCharacters/PhasePlayerCharacter_Climber.PhasePlayerCharacter_Climber_C" (Transformation|GetActorTransform _output_get) "Undefined" 0 0))
          (Pawn|Possess (Game|GetPlayerController 0) _returnvalue)
          (CallFunction|SpawnAI))))
    (:then_1
      (bind _outactors_3 (Actor|GetAllActorsOfClass "/Game/Objects/Blueprints/BP_Interacts/BP_MovingPlatform.BP_MovingPlatform_C"))
      (for _array_element_3 _outactors_3
        (Default|StarterLocation _array_element_3)))
    (:then_2
      (Development|PrintString "Hello")
      (bind _outactors_4 (Actor|GetAllActorsOfClass "/Game/Objects/Blueprints/BP_Interacts/BP_PressurePlate.BP_PressurePlate_C"))
      (for _array_element_4 _outactors_4
        (Default|Reset01 _array_element_4)))))

(event Custom|SpawnAI
  ;[1 1 1] Spawn AI
  (Utilities|FlowControl|Delay 0.2)
  (bind _outactors (Actor|GetAllActorsOfClass "/Game/Objects/Blueprints/Logic/SpawnersAI.SpawnersAI_C"))
  (for _array_element _outactors
    (AI|SpawnAIFromClass "/Game/Characters/Animals/BP_AnimalBase.BP_AnimalBase_C" 0 (Transformation|GetWorldLocation (Variables|/Game/Objects/Blueprints/Logic/SpawnersAI.SpawnersAI_C|GetDefaultSceneRoot _array_element)) "0, 0, 0" false)))

(event EventBeginPlay
  ;[1 1 1] Begin Play create Keycard widget
  (bind _returnvalue (UserInterface|CreateWidget "/Game/Objects/Widgets/Keycard_Widgets.Keycard_Widgets_C" (Game|GetPlayerController 0)))
  (UserInterface|Viewport|AddtoViewport _returnvalue 0)
  (CallFunction|SpawnAI)
  (Development|PrintString "Hello")
  (Utilities|FlowControl|Delay 2.0)
  (Variables|Default|SetGameJustStarted true))

(event EventOnRestartPlayer
  (params (NewPlayer :type Controller%20Object%20Reference))
  (bind _inventoryref (Variables|Default|GetInventoryRef))
  ;[1 1 1] Setting All variables back on respawning Playr
  (Utilities|IsValid NewPlayer
    (:Is%20Valid
      (bind _asphase_player_character (Utilities|Casting|CastToPhasePlayerCharacter (Game|GetPlayerCharacter 0)))
      (Variables|/Game/BlueprintCharacters/PhasePlayerCharacter.PhasePlayerCharacter_C|SetInventory _asphase_player_character _inventoryref)
      (bind _output_get (Variables|Default|SetInHand (Utilities|Array|Get(acopy) _inventoryref)))
      (Variables|/Game/BlueprintCharacters/PhasePlayerCharacter.PhasePlayerCharacter_C|SetItemInHand _asphase_player_character _output_get)
      (Variables|/Game/BlueprintCharacters/PhasePlayerCharacter.PhasePlayerCharacter_C|SetKeyCard01 _asphase_player_character (Variables|Default|GetKeycard01Ref))
      (if (Variables|Default|GetTimerDone?)
        (Variables|Default|SetTimerDone? false)
        (Variables|Default|SetMinutes 0)
        (Variables|Default|SetSeconds 20)))))

(fn ConstructionScript)