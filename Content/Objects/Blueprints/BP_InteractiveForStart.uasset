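; Interactive start checkpoint that, on Interact, switches every BP_InteractiveCheckPoint actor off and itself on.
; Activation spawns impulse, fire and charge particles at arrow components, then a delayed timeline flickers the spotlight and makes the trigger ignore pawns.
; The construction script sets text, sparkles and light from the On/Off state, while Tick refreshes them through a half-second Delay, zeroing the light only when off.
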(event Custom|StoreCheckPoint
  (params (Target :type Object%20Object%20Reference))
  (bind _chargeemitterloc (Variables|Default|GetChargeEmitterLoc))
  (bind _outactors (Actor|GetAllActorsOfClass "/Game/Objects/Blueprints/BP_InteractiveCheckPoint.BP_InteractiveCheckPoint_C"))
  (for _array_element _outactors
    (Variables|/Game/Objects/Blueprints/BP_InteractiveCheckPoint.BP_InteractiveCheckPoint_C|SetOnOffState _array_element "NewEnumerator1"))
  (Variables|Default|SetOnOffState "NewEnumerator0")
  (CallFunction|SpawnEmitter _chargeemitterloc "/Game/AVFX/Assets/Effects/P_Impulse.P_Impulse")
  (CallFunction|SpawnEmitter _chargeemitterloc "/Game/AVFX/Assets/Effects/P_Fire.P_Fire")
  (CallFunction|SpawnEmitter _chargeemitterloc "/Game/AVFX/Assets/Effects/P_Charge.P_Charge")
  (CallFunction|SpawnEmitter (Variables|Default|GetBaseChargeEmitterLoc) "/Game/AVFX/Assets/Effects/P_Charge.P_Charge")
  (Utilities|FlowControl|Delay 1.0)
  (bind _flicker (Timeline|Flicker PlayFromStart)
    (:Update
      (Rendering|Components|Light|SetIntensity (Variables|Default|GetSpotLight) _flicker)
      (Collision|SetCollisionResponsetoChannel (Variables|Default|GetTrigger) "ECC_Pawn" "ECR_Ignore"))))

(event EventTick
  (params (DeltaSeconds :type Float%20%28single-precision%29))
  (bind _text (Variables|Default|GetText))
  (bind _sparkles (Variables|Default|GetSparkles))
  (Utilities|FlowControl|Delay 0.5)
  (switch Utilities|FlowControl|Switch|SwitchonE_OnOFfStates (Variables|Default|GetOnOffState)
    (:NewEnumerator0
      (Rendering|Components|TextRender|SetText _text (Utilities|Text|MakeLiteralText "ON"))
      (Rendering|SetVisibility _sparkles true false))
    (:NewEnumerator1
      (Rendering|Components|TextRender|SetText _text (Utilities|Text|MakeLiteralText "Off"))
      (Rendering|SetVisibility _sparkles false false)
      (Rendering|Components|Light|SetIntensity (Variables|Default|GetSpotLight) 0.0))))

(fn ConstructionScript
  (bind _text (Variables|Default|GetText))
  (bind _sparkles (Variables|Default|GetSparkles))
  (bind _spotlight (Variables|Default|GetSpotLight))
  (switch Utilities|FlowControl|Switch|SwitchonE_OnOFfStates (Variables|Default|GetOnOffState)
    (:NewEnumerator0
      (Rendering|Components|TextRender|SetText _text (Utilities|Text|MakeLiteralText "ON"))
      (Rendering|SetVisibility _sparkles true false)
      (Rendering|Components|Light|SetIntensity _spotlight 5e+02))
    (:NewEnumerator1
      (Rendering|Components|TextRender|SetText _text (Utilities|Text|MakeLiteralText "Off"))
      (Rendering|SetVisibility _sparkles false false)
      (Rendering|Components|Light|SetIntensity _spotlight 0.0))))

(fn SpawnEmitter
  (params (ArrowComponent :type Arrow%20Component%20Object%20Reference) (Emitter :type Particle%20System%20Object%20Reference))
  (bind _returnvalue (Transformation|GetWorldTransform ArrowComponent))
  (Effects|SpawnEmitteratLocation Emitter (.location _returnvalue) (.rotation _returnvalue) (.scale _returnvalue)))

(fn Interact
  (params (TargetPoint :type Scene%20Component%20Object%20Reference) (Actor :type Actor%20Object%20Reference))
  (CallFunction|StoreCheckPoint TargetPoint)
  (return false))