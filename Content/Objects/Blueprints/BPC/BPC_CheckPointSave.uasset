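; BPC_CheckPointSave is a component that respawns the first player at an active checkpoint after resetting the level.
; ResSpawn finds the first BP_InteractiveCheckPoint in the active on/off state and does nothing if none matches.
; If GM_ShooterGuy's TimerDone is set, it restarts the player at the first PlayerStart instead.
; The component's event graph never triggers ResSpawn, and an alternative GM_Tester cast is left disconnected.
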(fn ResSpawn
  (bind _returnvalue (Game|GetPlayerController 0))
  (bind _returnvalue_2 (Game|GetGameMode))
  (bind _outactors (Actor|GetAllActorsOfClass "/Game/Objects/Blueprints/BP_InteractiveCheckPoint.BP_InteractiveCheckPoint_C"))
  (bind _array_element (Utilities|Array|ForEachLoopwithBreak _outactors :!label _label)
    (:LoopBody
      (if (Utilities|Enum|Equal(Enum) (Variables|/Game/Objects/Blueprints/BP_InteractiveCheckPoint.BP_InteractiveCheckPoint_C|GetOnOffState _array_element) "NewEnumerator0")
        (Variables|Default|SetOneIsActive? true)
        (goto _label Break)))
    (:Completed
      (if (Variables|Default|GetOneIsActive?)
        (bind _output_get (Variables|Default|SetCheckPoints _array_element))
        (bind _asgm_shooter_guy (Utilities|Casting|CastToGM_ShooterGuy _returnvalue_2))
        (if (Variables|/Game/Objects/GamModes/GM_ShooterGuy.GM_ShooterGuy_C|GetTimerDone? _asgm_shooter_guy)
          (bind _outactors_2 (Actor|GetAllActorsOfClass "/Script/Engine.PlayerStart"))
          (Class|GameModeBase|ResetLevel _returnvalue_2)
          (Class|GameModeBase|RestartPlayeratPlayerStart _returnvalue_2 _returnvalue (Utilities|Array|Get(acopy) _outactors_2))
          (Variables|Default|SetOneIsActive? false)
          (else
            (Class|GameModeBase|ResetLevel _returnvalue_2)
            (Class|GameModeBase|RestartPlayeratPlayerStart _returnvalue_2 _returnvalue _output_get)
            (Variables|Default|SetOneIsActive? false)))))))