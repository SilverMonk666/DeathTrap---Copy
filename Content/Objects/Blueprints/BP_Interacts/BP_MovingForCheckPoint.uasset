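; Moving platform Blueprint that travels between its starting position and an EndPoint component, likely tied to checkpoints.
; BeginPlay caches both world locations and sets the timeline play rate from a variable.
; Each MovePlatform call flip-flops the timeline between playing forward and reversing, lerping the platform's location with sweep enabled.
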(event Custom|MovePlatform
  (Utilities|FlowControl|FlipFlop
    (:A
      (bind _moveplat (Timeline|MovePlat Play)
        (:Update
          (Transformation|SetWorldLocation (Variables|Default|GetPlatform) (Math|Vector|Lerp(Vector) (Variables|Default|GetStartlocation) (Variables|Default|GetEndPointLocation) _moveplat) true false))))
    (:B
      (Timeline|MovePlat Reverse))))

(event EventBeginPlay
  (Variables|Default|SetStartlocation (Transformation|GetWorldLocation (Variables|Default|GetPlatform)))
  (Variables|Default|SetEndPointLocation (Transformation|GetWorldLocation (Variables|Default|GetEndPoint)))
  (Components|Timeline|SetPlayRate (Variables|Default|GetMovePlat) (Variables|Default|GetPlayRate)))

(fn ConstructionScript)