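; Moving hazard that respawns any Character overlapping either of its two triggers through the checkpoint save component's ResSpawn.
; Two timelines shuttle Trigger endlessly between the Cube and EndPoint positions captured at BeginPlay, setting its rotation and pausing at each end.
; The configurable play rate applies only to the outbound timeline.
; An unconnected checkpoint-search chain is left in the graph and never runs.
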(event OnComponentBeginOverlap(Trigger)
  (params (OverlappedComponent :type Primitive%20Component%20Object%20Reference) (OtherActor :type Actor%20Object%20Reference) (OtherComp :type Primitive%20Component%20Object%20Reference) (OtherBodyIndex :type Integer) (bFromSweep :type Boolean) (SweepResult :type Hit%20Result%20Structure%20%28by%20ref%29))
  (Utilities|Casting|CastToCharacter (stale OnComponentBeginOverlap(tRIGGER02) OtherActor))
  (Default|ResSpawn (Variables|Default|GetBPC_CheckPointSave)))

(event OnComponentBeginOverlap(tRIGGER02)
  (params (OverlappedComponent :type Primitive%20Component%20Object%20Reference) (OtherActor :type Actor%20Object%20Reference) (OtherComp :type Primitive%20Component%20Object%20Reference) (OtherBodyIndex :type Integer) (bFromSweep :type Boolean) (SweepResult :type Hit%20Result%20Structure%20%28by%20ref%29))
  (Utilities|Casting|CastToCharacter OtherActor)
  (Default|ResSpawn (Variables|Default|GetBPC_CheckPointSave)))

(event Custom|Reverse
  (bind _moveplat (Timeline|MovePlatform PlayFromStart)
    (:Update
      (Transformation|SetWorldLocation (Variables|Default|GetTrigger) (Math|Vector|Lerp(Vector) (Variables|Default|GetStartLocation) (Variables|Default|GetEndLocation) _moveplat) false false))
    (:Finished
      (Transformation|SetWorldRotation (Variables|Default|GetTrigger) "0,-180.000000, 0" false false)
      (Utilities|FlowControl|Delay (Variables|Default|GetDelayBeforeNextMove))
      (bind _moveplat_2 (Timeline|Timeline_0 PlayFromStart)
        (:Update
          (Transformation|SetWorldLocation (Variables|Default|GetTrigger) (Math|Vector|Lerp(Vector) (Variables|Default|GetEndLocation) (Variables|Default|GetStartLocation) _moveplat_2) false false))
        (:Finished
          (Utilities|FlowControl|Delay (Variables|Default|GetDelayBeforeNextMove))
          (CallFunction|Reverse)
          (Transformation|SetWorldRotation (Variables|Default|GetTrigger) "0.000000,180.000000,0.000000" false false))))))

(event EventBeginPlay
  (Variables|Default|SetStartLocation (Transformation|GetWorldLocation (Variables|Default|GetCube)))
  (Variables|Default|SetEndLocation (Transformation|GetWorldLocation (Variables|Default|GetEndPoint)))
  (Components|Timeline|SetPlayRate (Variables|Default|GetMovePlatform) (Variables|Default|GetPlayRate))
  (bind _moveplat (Timeline|MovePlatform Play)
    (:Update
      (Transformation|SetWorldLocation (Variables|Default|GetTrigger) (Math|Vector|Lerp(Vector) (Variables|Default|GetStartLocation) (Variables|Default|GetEndLocation) _moveplat) false false))
    (:Finished
      (Transformation|SetWorldRotation (Variables|Default|GetTrigger) "0,-180.000000, 0" false false)
      (Utilities|FlowControl|Delay (Variables|Default|GetDelayBeforeNextMove))
      (bind _moveplat_2 (Timeline|Timeline_0 PlayFromStart)
        (:Update
          (Transformation|SetWorldLocation (Variables|Default|GetTrigger) (Math|Vector|Lerp(Vector) (Variables|Default|GetEndLocation) (Variables|Default|GetStartLocation) _moveplat_2) false false))
        (:Finished
          (Utilities|FlowControl|Delay (Variables|Default|GetDelayBeforeNextMove))
          (CallFunction|Reverse)
          (Transformation|SetWorldRotation (Variables|Default|GetTrigger) "0.000000,180.000000,0.000000" false false))))))

(fn ConstructionScript)