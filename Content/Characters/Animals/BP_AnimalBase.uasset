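; Base animal character that chases the player and kills them when its capsule overlaps them.
; Overlap events on component R tell its controller (PlayerCharacterControllerBase) to Follow when the player enters, and to Wander and set ConLoop when they leave.
; A FollowPlayer event also triggers Follow directly.
; Interact is a stub returning false, and a checkpoint respawn call is left unconnected.
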(event OnComponentBeginOverlap(CapsuleComponent)
  (params (OverlappedComponent :type Primitive%20Component%20Object%20Reference) (OtherActor :type Actor%20Object%20Reference) (OtherComp :type Primitive%20Component%20Object%20Reference) (OtherBodyIndex :type Integer) (bFromSweep :type Boolean) (SweepResult :type Hit%20Result%20Structure%20%28by%20ref%29))
  (bind _asphase_player_character (Utilities|Casting|CastToPhasePlayerCharacter OtherActor))
  (Default|KillPlayer _asphase_player_character))

(event OnComponentBeginOverlap(r)
  (params (OverlappedComponent :type Primitive%20Component%20Object%20Reference) (OtherActor :type Actor%20Object%20Reference) (OtherComp :type Primitive%20Component%20Object%20Reference) (OtherBodyIndex :type Integer) (bFromSweep :type Boolean) (SweepResult :type Hit%20Result%20Structure%20%28by%20ref%29))
  (Utilities|Casting|CastToPhasePlayerCharacter OtherActor)
  (bind _asplayer_character_controller_base (Utilities|Casting|CastToPlayerCharacterControllerBase (Pawn|GetController)))
  (Default|Follow _asplayer_character_controller_base))

(event OnComponentEndOverlap(r)
  (params (OverlappedComponent :type Primitive%20Component%20Object%20Reference) (OtherActor :type Actor%20Object%20Reference) (OtherComp :type Primitive%20Component%20Object%20Reference) (OtherBodyIndex :type Integer))
  (Utilities|Casting|CastToPhasePlayerCharacter OtherActor)
  (bind _asplayer_character_controller_base (Utilities|Casting|CastToPlayerCharacterControllerBase (Pawn|GetController)))
  (Default|Wander _asplayer_character_controller_base)
  (Variables|/Game/Characters/Animals/PlayerCharacterControllerBase.PlayerCharacterControllerBase_C|SetConLoop _asplayer_character_controller_base true))

(event Custom|FollowPlayer
  (params (ActorRef :type Actor%20Object%20Reference))
  (bind _asplayer_character_controller_base (Utilities|Casting|CastToPlayerCharacterControllerBase (Pawn|GetController)))
  (Default|Follow _asplayer_character_controller_base))

(event EventBeginPlay)

(event Collision|EventActorBeginOverlap
  (params (OtherActor :type Actor%20Object%20Reference)))

(event EventTick
  (params (DeltaSeconds :type Float%20%28single-precision%29)))

(fn ConstructionScript)

(fn Interact
  (params (Actor :type Actor%20Object%20Reference) (TargetPoint :type Scene%20Component%20Object%20Reference))
  (return false))